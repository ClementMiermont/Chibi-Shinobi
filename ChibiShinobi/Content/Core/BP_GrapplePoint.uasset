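; Grapple point actor that shows the player a detection widget while activated and tracks whether it has been used.
; While active and unused, Tick scales the widget's fill by player distance, between detection radius and throw distance, turning it green within throw range.
; Use plays the node animation and stops those updates.
; The Box overlap disables Detection collision while the player is inside, then restores it and re-arms the point on exit.
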(event `self.ReceiveBeginPlay`
  (`|ExecutionSequence`
    (:`then_0`
      (bind _aswbp_detection_node (cast `/Game/Core/WBP_DetectionNode` (`WidgetComponent.GetUserWidgetObject` (`self.Widget`))))
      (set `self.Widget Ref` _aswbp_detection_node))
    (:`then_1`
      (bind _asbp_third_person_character (cast `/Game/Core/BP_ThirdPersonCharacter` (`GameplayStatics.GetPlayerPawn` 0)))
      (set `self.PlayerRef2` _asbp_third_person_character))))

(event `self.ReceiveTick`
  (params (DeltaSeconds :type "Float (single-precision)"))
  (if (and (`self.bActive`) (not (`self.Used`)))
    (`self.CheckDistanceFromPlayer`)))

(event `self.Box.OnComponentBeginOverlap`
  (params (OverlappedComponent :type "PrimitiveComponent Object Reference") (OtherActor :type "Actor Object Reference") (OtherComp :type "PrimitiveComponent Object Reference") (OtherBodyIndex :type Integer) (bFromSweep :type Boolean) (SweepResult :type "HitResult Structure (by ref)"))
  (if (== OtherActor (`self.PlayerRef2`))
    (`PrimitiveComponent.SetCollisionEnabled` (`self.Detection`) "NoCollision")))

(event `self.Box.OnComponentEndOverlap`
  (params (OverlappedComponent :type "PrimitiveComponent Object Reference") (OtherActor :type "Actor Object Reference") (OtherComp :type "PrimitiveComponent Object Reference") (OtherBodyIndex :type Integer))
  (if (== OtherActor (`self.PlayerRef2`))
    (`PrimitiveComponent.SetCollisionEnabled` (`self.Detection`) "QueryAndPhysics")
    (`self.Reactivate`)))

(fn `Activate`
  (params (Player :type "/Game/Core/BP_ThirdPersonCharacter Object Reference"))
  (set `self.bActive` true)
  (`Widget.SetVisibility` (`self.Widget Ref`) "Visible")
  (set `self.PlayerRef2` Player))

(fn `CheckDistanceFromPlayer`
  (bind _playerref2 (`self.PlayerRef2`))
  (bind _returnvalue (`KismetMathLibrary.MapRangeClamped` (`KismetMathLibrary.VSize` (- (`self.K2_GetActorLocation` (`self.PlayerRef2`)) (`self.K2_GetActorLocation`))) (`/Game/Core/BP_ThirdPersonCharacter.GrappleThrowDistance` _playerref2) (`/Game/Core/BP_ThirdPersonCharacter.DetectionRadius` _playerref2) 80.0 10.0))
  (`Image.SetDesiredSizeOverride` (`/Game/Core/WBP_DetectionNode.Filling` (`self.Widget Ref`)) (`KismetMathLibrary.MakeVector2D` _returnvalue _returnvalue))
  (`Image.SetColorAndOpacity` (`/Game/Core/WBP_DetectionNode.Filling` (`self.Widget Ref`)) (select `bool` (== _returnvalue 80.0) :`false` (struct :`R` 0.244792 :`G` 0.244792 :`B` 0.244792 :`A` 1.0) :`true` (struct :`R` 0.1841 :`G` 0.630208 :`B` 0.206321 :`A` 1.0) :!type "LinearColor Structure")))

(fn `Deactivate`
  (set `self.bActive` false)
  (`Widget.SetVisibility` (`self.Widget Ref`) "Hidden"))

(fn `Reactivate`
  (set `self.Used` false))

(fn `Use`
  (bind _widget_ref (`self.Widget Ref`))
  (set `self.Used` true)
  (`UserWidget.PlayAnimation` _widget_ref (`/Game/Core/WBP_DetectionNode.NodeUse` _widget_ref) 0.0 1 "Forward" 1.0 true))

(fn `UserConstructionScript`)